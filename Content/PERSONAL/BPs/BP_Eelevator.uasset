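; Elevator actor that carries its cabin between floors chosen by the first-person player.
; Interract shows the mouse cursor, passes floor limits to the character's ElevatorRoom and stores that character for SecondInterract to read the requested floor.
; For a valid new floor, chained timelines swing both doors shut, lerp the root Z by a fixed height per floor, then reopen the doors.
; A NotMoving flag blocks input during travel.
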(event `self.ReceiveBeginPlay`
  (set `self.Door1 RelativeRotation` (`SceneComponent.RelativeRotation` (`self.LiftDoor1`)))
  (set `self.Door2 RelativeRotation` (`SceneComponent.RelativeRotation` (`self.LiftDoor2`)))
  (set `self.WorldLocationLift` (`SceneComponent.K2_GetComponentLocation` (`self.Scene`))))

(event `/Game/PERSONAL/BPs/BPI_Interract.Interract`
  (params (BP_FirstPersonCharacter :type "/Game/FirstPerson/Blueprints/BP_FirstPersonCharacter Object Reference"))
  (if (`self.NotMoving`)
    (set `PlayerController.bShowMouseCursor` true (`GameplayStatics.GetPlayerController` 0))
    (set `/Game/FirstPerson/Blueprints/BP_FirstPersonCharacter.MaxFloor` (`self.MaxElevatorFloors`) BP_FirstPersonCharacter)
    (set `/Game/FirstPerson/Blueprints/BP_FirstPersonCharacter.CurrentFloor` (`self.FloorYoureAt`) BP_FirstPersonCharacter)
    (`/Game/FirstPerson/Blueprints/BP_FirstPersonCharacter.ElevatorRoom?` BP_FirstPersonCharacter)
    (set `self.CurrentPlayer` BP_FirstPersonCharacter)))

(event `/Game/PERSONAL/BPs/BPI_Interract.SecondInterract`
  (bind (_door1_relativerotation_roll _door1_relativerotation_pitch _door1_relativerotation_yaw) (`KismetMathLibrary.BreakRotator` (`self.Door1 RelativeRotation`)))
  (bind (_door2_relativerotation_roll _door2_relativerotation_pitch _door2_relativerotation_yaw) (`KismetMathLibrary.BreakRotator` (`self.Door2 RelativeRotation`)))
  (bind (_door1_relativerotation_roll_2 _door1_relativerotation_pitch_2 _door1_relativerotation_yaw_2) (`KismetMathLibrary.BreakRotator` (`self.Door1 RelativeRotation`)))
  (bind (_door2_relativerotation_roll_2 _door2_relativerotation_pitch_2 _door2_relativerotation_yaw_2) (`KismetMathLibrary.BreakRotator` (`self.Door2 RelativeRotation`)))
  (bind (_worldlocationlift_x _worldlocationlift_y _worldlocationlift_z) (`KismetMathLibrary.BreakVector` (`self.WorldLocationLift`)))
  (bind _new_elevator_floor (`self.New Elevator Floor`))
  (bind _returnvalue (+ _worldlocationlift_z (* (- (`self.New Elevator Floor`) (`self.FloorYoureAt`)) 500)))
  (bind _output_get (set `self.New Elevator Floor` (`/Game/FirstPerson/Blueprints/BP_FirstPersonCharacter.NewElevatorFloor` (`self.CurrentPlayer`))))
  (if (and (!= _output_get (`self.FloorYoureAt`)) (>= _new_elevator_floor 0) (<= _new_elevator_floor (`self.MaxElevatorFloors`)))
    (if (`self.NotMoving`)
      (set `self.NotMoving` false)
      (bind (_direction _newtrack_0) (`Timeline|DoorClosing` :!via `PlayFromStart`)
        (:`Update`
          (bind _returnvalue_2 (`KismetMathLibrary.Lerp` 0.0 30.0 _newtrack_0))
          (`SceneComponent.K2_SetRelativeRotation` (`self.LiftDoor1`) (`KismetMathLibrary.MakeRotator` _door1_relativerotation_roll_2 _door1_relativerotation_pitch_2 (+ _door1_relativerotation_yaw_2 _returnvalue_2)) false false)
          (`SceneComponent.K2_SetRelativeRotation` (`self.LiftDoor2`) (`KismetMathLibrary.MakeRotator` _door2_relativerotation_roll_2 _door2_relativerotation_pitch_2 (- _door2_relativerotation_yaw_2 _returnvalue_2)) false false))
        (:`Finished`
          (bind (_direction_2 _newtrack_0_2) (`Timeline|Timeline` :!via `PlayFromStart`)
            (:`Update`
              (`SceneComponent.K2_SetWorldLocation` (`self.Scene`) (`KismetMathLibrary.MakeVector` _worldlocationlift_x _worldlocationlift_y (`KismetMathLibrary.Lerp` _worldlocationlift_z _returnvalue _newtrack_0_2)) false false))
            (:`Finished`
              (set `self.WorldLocationLift` (`KismetMathLibrary.MakeVector` _worldlocationlift_x _worldlocationlift_y _returnvalue))
              (set `self.FloorYoureAt` (`self.New Elevator Floor`))
              (bind (_direction_3 _newtrack_0_3) (`Timeline|Timeline_0` :!via `ReverseFromEnd`)
                (:`Update`
                  (bind _returnvalue_3 (`KismetMathLibrary.Lerp` 0.0 30.0 _newtrack_0_3))
                  (`SceneComponent.K2_SetRelativeRotation` (`self.LiftDoor1`) (`KismetMathLibrary.MakeRotator` _door1_relativerotation_roll _door1_relativerotation_pitch (+ _door1_relativerotation_yaw _returnvalue_3)) false false)
                  (`SceneComponent.K2_SetRelativeRotation` (`self.LiftDoor2`) (`KismetMathLibrary.MakeRotator` _door2_relativerotation_roll _door2_relativerotation_pitch (- _door2_relativerotation_yaw _returnvalue_3)) false false))
                (:`Finished`
                  (set `self.NotMoving` true))))))))))

(fn `UserConstructionScript`)