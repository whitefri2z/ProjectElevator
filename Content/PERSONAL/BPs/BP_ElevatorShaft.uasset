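; Elevator shaft actor that builds a multi-storey shaft with floors and a working elevator at runtime.
; On BeginPlay, only when IsParent is set, it spawns a base floor, then loops up to NumberOfFloors, stacking child shaft segments and offset floors at fixed height intervals from the LiftShaft transform.
; It finally spawns the elevator at the shaft's transform and passes NumberOfFloors as its maximum floor.
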(event `self.ReceiveBeginPlay`
  (bind _numberoffloorsdone (`self.NumberOfFloorsDone`))
  (bind _returnvalue (`SceneComponent.K2_GetComponentToWorld` (`self.LiftShaft`)))
  (bind _returnvalue_2 (+ (.z (.location _returnvalue)) (* (`self.NumberOfFloorsDone`) 500)))
  (bind _returnvalue_3 (`KismetMathLibrary.MakeTransform` (`KismetMathLibrary.MakeVector` (- (.x (.location _returnvalue)) 120.0) (+ (.y (.location _returnvalue)) 320.0) _returnvalue_2) (.rotation _returnvalue) (.scale _returnvalue)))
  (if (`self.IsParent`)
    (`|SpawnActorFromClass` "/Game/PERSONAL/BPs/BP_Floor.BP_Floor_C" _returnvalue_3 "AdjustIfPossibleButAlwaysSpawn" "MultiplyWithRoot" null null)
    (while (!= (>= _numberoffloorsdone (`self.NumberOfFloors`)) true)
      (`/Engine/EditorBlueprintResources/StandardMacros.IncrementInt` _numberoffloorsdone
        (:`  `
          (`|SpawnActorFromClass` "/Game/PERSONAL/BPs/BP_ElevatorShaftChild.BP_ElevatorShaftChild_C" (`KismetMathLibrary.MakeTransform` (`KismetMathLibrary.MakeVector` (.x (.location _returnvalue)) (.y (.location _returnvalue)) _returnvalue_2) (.rotation _returnvalue) (.scale _returnvalue)) "AdjustIfPossibleButAlwaysSpawn" "MultiplyWithRoot" null null)
          (`|SpawnActorFromClass` "/Game/PERSONAL/BPs/BP_Floor.BP_Floor_C" _returnvalue_3 "AdjustIfPossibleButAlwaysSpawn" "MultiplyWithRoot" null null))))
    (bind _returnvalue_4 (`|SpawnActorFromClass` "/Game/PERSONAL/BPs/BP_Eelevator.BP_Eelevator_C" (`SceneComponent.K2_GetComponentToWorld` (`self.LiftShaft`)) "Undefined" "MultiplyWithRoot" null null))
    (set `/Game/PERSONAL/BPs/BP_Eelevator.MaxElevatorFloors` (`self.NumberOfFloors`) _returnvalue_4)))

(fn `UserConstructionScript`)